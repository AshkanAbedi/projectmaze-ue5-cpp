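; Main character Blueprint that sets up player input, with an unfinished, disconnected laser aiming feature.
; On BeginPlay it enables input for the first player controller and adds the IM_Context Enhanced Input mapping context.
; Unwired aiming logic would debug-trace forward from LaserPoint and align it to the CameraBoom target rotation, but it never runs.
; Tick, overlap and construction script are empty.
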(event `self.ReceiveBeginPlay`
  (bind _returnvalue (`GameplayStatics.GetPlayerController` 0))
  (`self.EnableInput` _returnvalue)
  (message `EnhancedInputSubsystemInterface.AddMappingContext` (pcsubsystem `EnhancedInputLocalPlayerSubsystem` _returnvalue) "/Game/Blueprint/IM_Context.IM_Context" 0 (struct)))

(event `self.ReceiveTick`
  (params (DeltaSeconds :type "Float (single-precision)")))

(fn `UserConstructionScript`)